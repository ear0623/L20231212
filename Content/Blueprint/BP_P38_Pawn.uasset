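; BP_P38_Pawn is a player-controlled P-38 plane pawn that constantly flies forward along its actor forward vector.
; Pitch and Roll axes rotate it locally, scaled by delta time and RotateSpeed, while Fire spawns BP_Rocket using the Body's Missile socket transform in parent-bone space.
; BeginPlay registers Left and Right with the BPRotateSecnes component.
; A RotatePropeller helper spins a given component, but nothing in this file calls it.
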(event `self.ReceiveBeginPlay`
  (`KismetArrayLibrary.Array_Add` (`/Game/Blueprint/BP_RotateScenes.SceneComponents` (`self.BP_RotateSecnes`)) (`self.Left`))
  (`KismetArrayLibrary.Array_Add` (`/Game/Blueprint/BP_RotateScenes.SceneComponents` (`self.BP_RotateSecnes`)) (`self.Right`)))

(event `self.ReceiveTick`
  (params (DeltaSeconds :type "Float (single-precision)"))
  (`self.AddMovementInput` (`self.GetActorForwardVector`)))

(event `InputAxis|Pitch`
  (params (AxisValue :type "Float (single-precision)"))
  (`self.K2_AddActorLocalRotation` (`KismetMathLibrary.MakeRotator` 0.0 (* AxisValue (`GameplayStatics.GetWorldDeltaSeconds`) (`self.RotateSpeed`)))))

(event `InputAxis|Roll`
  (params (AxisValue :type "Float (single-precision)"))
  (`self.K2_AddActorLocalRotation` (`KismetMathLibrary.MakeRotator` (* AxisValue (`GameplayStatics.GetWorldDeltaSeconds`) (`self.RotateSpeed`)))))

(event `InputAction|Fire`
  (params (Key :type "Key Structure"))
  (:`Pressed`
    (`|SpawnActorFromClass` "/Game/Blueprint/Kidding/BP_Rocket.BP_Rocket_C" (`SceneComponent.GetSocketTransform` (`self.Body`) "Missile" "RTS_ParentBoneSpace") "Undefined" "MultiplyWithRoot" null null)))

(fn `RotatePropeller`
  (params (self2 :type "SceneComponent Object Reference"))
  (`SceneComponent.K2_AddLocalRotation` self2 (`KismetMathLibrary.MakeRotator` (* (`GameplayStatics.GetWorldDeltaSeconds`) (`self.PropeellerRotationSpeed`))) false false))

(fn `UserConstructionScript`)