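; BP_P38 is a P-38 plane actor that drifts steadily along world X, scaled by frame time on Tick.
; On BeginPlay it adds its Left and Right components to the BPRotateSecnes SceneComponents list.
; A RotatePropeller function spins a given component in roll at PropeellerRotationSpeed but is not called in this Blueprint.
; Registering itself with BPAddMoveScenes is present but unwired, so the actor handles its own movement.
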(event `self.ReceiveBeginPlay`
  (`KismetArrayLibrary.Array_Add` (`/Game/Blueprint/BP_RotateScenes.SceneComponents` (`self.BP_RotateSecnes`)) (`self.Left`))
  (`KismetArrayLibrary.Array_Add` (`/Game/Blueprint/BP_RotateScenes.SceneComponents` (`self.BP_RotateSecnes`)) (`self.Right`)))

(event `self.ReceiveTick`
  (params (DeltaSeconds :type "Float (single-precision)"))
  (`self.K2_AddActorWorldOffset` (`KismetMathLibrary.MakeVector` (* (`GameplayStatics.GetWorldDeltaSeconds`) 10.0))))

(fn `RotatePropeller`
  (params (self2 :type "SceneComponent Object Reference"))
  (`SceneComponent.K2_AddLocalRotation` self2 (`KismetMathLibrary.MakeRotator` (* (`GameplayStatics.GetWorldDeltaSeconds`) (`self.PropeellerRotationSpeed`))) false false))

(fn `UserConstructionScript`)